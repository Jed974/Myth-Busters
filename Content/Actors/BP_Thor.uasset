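; BP_Thor is the actor for the flying god Thor, driven by a GodMovement component.
; Each tick it turns the skeletal mesh left or right by the facing flag and feeds velocity, as a percentage of max fly speeds, to AnimBP_Thor.
; Horizontal speed is passed unsigned and vertical speed signed.
; Capsule hits only fire a debug-drawn line trace along the impact normal, with the result unused.
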(event OnComponentBeginOverlap(CapsuleComponent)
  (params (OverlappedComponent :type Primitive%20Component%20Object%20Reference) (OtherActor :type Actor%20Object%20Reference) (OtherComp :type Primitive%20Component%20Object%20Reference) (OtherBodyIndex :type Integer) (bFromSweep :type Boolean) (SweepResult :type Hit%20Result%20Structure%20%28by%20ref%29)))

(event OnComponentHit(CapsuleComponent)
  (params (HitComponent :type Primitive%20Component%20Object%20Reference) (OtherActor :type Actor%20Object%20Reference) (OtherComp :type Primitive%20Component%20Object%20Reference) (NormalImpulse :type Vector :default "0, 0, 0") (Hit :type Hit%20Result%20Structure%20%28by%20ref%29))
  (bind (_bblockinghit _binitialoverlap _time _distance _location _impactpoint _normal) (Collision|BreakHitResult Hit))
  (Collision|LineTraceByChannel _impactpoint (+ _impactpoint (* _normal 1e+02)) "TraceTypeQuery1" false 0 "ForDuration"))

(event EventBeginPlay
  (bind _asanim_bp_thor (Utilities|Casting|CastToAnimBP_Thor (Components|SkeletalMesh|GetAnimInstance (Variables|Default|GetSkeletalMesh))))
  (Variables|Default|SetAnimInstance _asanim_bp_thor))

(event Collision|EventActorBeginOverlap
  (params (OtherActor :type Actor%20Object%20Reference)))

(event EventTick
  (params (DeltaSeconds :type Float%20%28single-precision%29))
  (bind _skeletalmesh (Variables|Default|GetSkeletalMesh))
  (bind _animinstance (Variables|Default|GetAnimInstance))
  (bind _godmovement (Variables|Default|GetGodMovement))
  (bind _velocity (Variables|/Script/MythBusters.GodMovementComponent|GetVelocity _godmovement))
  (bind (_x _y) (Math|Vector2D|BreakVector2D _velocity))
  ;[1 1 1] Flip
  (if (Variables|/Script/MythBusters.GodMovementComponent|GetisFacingRight (Variables|Default|GetGodMovement))
    (Transformation|SetRelativeRotation _skeletalmesh "0,-90.000000, 0" false false)
    (else
      (Transformation|SetRelativeRotation _skeletalmesh "0,90.000000, 0" false false)))
  (Variables|/Game/Animations/Thor/AnimBP_Thor.AnimBP_Thor_C|SetSpeedX _animinstance (* (/ (Math|Float|Absolute(Float) _x) (Variables|/Script/MythBusters.GodMovementComponent|GetMaxHorizontalFlySpeed _godmovement)) 1e+02))
  (Variables|/Game/Animations/Thor/AnimBP_Thor.AnimBP_Thor_C|SetSpeedY _animinstance (* (/ _y (Variables|/Script/MythBusters.GodMovementComponent|GetMaxVerticalFlySpeed _godmovement)) 1e+02)))

(fn ConstructionScript)